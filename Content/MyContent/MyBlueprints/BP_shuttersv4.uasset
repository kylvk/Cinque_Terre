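; Shutter actor that randomizes the pose of a left and right shutter pivot for visual variety.
; The construction script calls RandomShutter, so the pose re-rolls whenever construction runs, with no active runtime logic.
; A weighted roll leaves both pivots at zero, flips both 180 degrees or, least often, gives each an independent partial yaw in opposite directions.
; A leftover debug print fires on every roll.
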(event Custom|RandomShutter
  (Development|PrintString "FUCKING WORKS")
  (Variables|Default|SetOpenPercentage (Math|Random|RandomFloatinRange 0.0 1.0))
  (if (< (Variables|Default|GetOpenPercentage) (Math|Float|MakeLiteralFloat 0.5))
    (Transformation|SetRelativeRotation (Variables|Default|Getleftpiv) "0, 0, 0" false false)
    (Transformation|SetRelativeRotation (Variables|Default|Getrightpiv) "0, 0, 0" false false)
    (elif (< (Variables|Default|GetOpenPercentage) (Math|Float|MakeLiteralFloat 0.85))
      (Transformation|SetRelativeRotation (Variables|Default|Getleftpiv) "0.000000,180.000000,0.000000" false false)
      (Transformation|SetRelativeRotation (Variables|Default|Getrightpiv) "0.000000,180.000000,0.000000" false false)
      (else
        (Transformation|SetRelativeRotation (Variables|Default|Getleftpiv) (Math|Rotator|MakeRotator 0.0 0.0 (Math|Random|RandomFloatinRange 1.0 179.0)) false false)
        (Transformation|SetRelativeRotation (Variables|Default|Getrightpiv) (Math|Rotator|MakeRotator 0.0 0.0 (Math|Random|RandomFloatinRange -1.0 -179.0)) false false)))))

(event EventBeginPlay)

(event Collision|EventActorBeginOverlap
  (params (OtherActor :type Actor%20Object%20Reference)))

(event EventTick
  (params (DeltaSeconds :type Float%20%28single-precision%29)))

(fn ConstructionScript
  (CallFunction|RandomShutter))