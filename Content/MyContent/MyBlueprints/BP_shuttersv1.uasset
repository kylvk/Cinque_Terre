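; Window shutter pair Blueprint that randomizes how its left and right shutters are posed, adding variety between placed copies.
; The Construction Script uses weighted random rolls to leave both at zero rotation, turn both to a half-turn yaw, or occasionally give each its own intermediate yaw.
; The rolls are unseeded, so poses can change whenever construction reruns.
; The event graph has no active logic.
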(event EventBeginPlay)

(event Collision|EventActorBeginOverlap
  (params (OtherActor :type Actor%20Object%20Reference)))

(event EventTick
  (params (DeltaSeconds :type Float%20%28single-precision%29)))

(fn ConstructionScript
  (bind _returnvalue (Math|Random|RandomFloatinRange 0.0 1.0))
  (if (< _returnvalue (Math|Float|MakeLiteralFloat 0.5))
    (Transformation|SetRelativeRotation (Variables|Default|GetShutterLeft) "0.000000,0.000000,0.000000" false false)
    (Transformation|SetRelativeRotation (Variables|Default|GetShutterRight) "0.000000,0.000000,0.000000" false false)
    (elif (< _returnvalue (Math|Float|MakeLiteralFloat 0.85))
      (Transformation|SetRelativeRotation (Variables|Default|GetShutterLeft) "180.000000,0.000000,0.000000" false false)
      (Transformation|SetRelativeRotation (Variables|Default|GetShutterRight) "180.000000,0.000000,0.000000" false false)
      (else
        (Transformation|SetRelativeRotation (Variables|Default|GetShutterLeft) (Math|Rotator|MakeRotator 0.0 0.0 (Math|Random|RandomFloatinRange 1.0 179.0)) false false)
        (Transformation|SetRelativeRotation (Variables|Default|GetShutterRight) (Math|Rotator|MakeRotator 0.0 0.0 (Math|Random|RandomFloatinRange 1.0 179.0)) false false)))))